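; Actor component that handles purchasable upgrades for click damage, shoot speed and atom value in what appears to be a clicker-style game.
; Each upgrade function changes its stat, charges the first-person character's currency component, counts the purchase and multiplies its next cost.
; Damage and currency multiplier live on the character's components, while shoot speed is stored here.
; A separate function checks affordability; the upgrades do not call it, and the scientists upgrade is empty.
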(fn UpgradeClickDMG
  (bind _asbp_first_person_character (Utilities|Casting|CastToBP_FirstPersonCharacter (Game|GetPlayerCharacter 0)))
  (Variables|/Game/Blueprints/AC_DamageSystem.AC_DamageSystem_C|Setdamage (Variables|/Game/FirstPerson/Blueprints/BP_FirstPersonCharacter.BP_FirstPersonCharacter_C|GetAC_DamageSystem _asbp_first_person_character) (+ (Variables|/Game/Blueprints/AC_DamageSystem.AC_DamageSystem_C|Getdamage (Variables|/Game/FirstPerson/Blueprints/BP_FirstPersonCharacter.BP_FirstPersonCharacter_C|GetAC_DamageSystem _asbp_first_person_character)) 1))
  (Variables|Default|SetclickDMGUpgrades (+ (Variables|Default|GetclickDMGUpgrades) 1))
  (Default|RemoveCurrency (Variables|/Game/FirstPerson/Blueprints/BP_FirstPersonCharacter.BP_FirstPersonCharacter_C|GetAC_Currency _asbp_first_person_character) (Variables|Default|GetclickDMGCost))
  (Variables|Default|SetclickDMGCost (* (Variables|Default|GetclickDMGCost) 1.1)))

(fn UpgradeShootSpeed
  (Variables|Default|SetshootSpeed (- (Variables|Default|GetshootSpeed) 0.005))
  (Variables|Default|SetshootSpeedUpgrades (+ (Variables|Default|GetshootSpeedUpgrades) 1))
  (bind _asbp_first_person_character (Utilities|Casting|CastToBP_FirstPersonCharacter (Game|GetPlayerCharacter 0)))
  (Default|RemoveCurrency (Variables|/Game/FirstPerson/Blueprints/BP_FirstPersonCharacter.BP_FirstPersonCharacter_C|GetAC_Currency _asbp_first_person_character) (Variables|Default|GetshootSpeedCost))
  (Variables|Default|SetshootSpeedCost (* (Variables|Default|GetshootSpeedCost) 2.5)))

(fn UpgradeScientists)

(fn UpgradeAtomValue
  (bind _asbp_first_person_character (Utilities|Casting|CastToBP_FirstPersonCharacter (Game|GetPlayerCharacter 0)))
  (Variables|/Game/Blueprints/AC_Currency.AC_Currency_C|SetcurrencyMultiplier (Variables|/Game/FirstPerson/Blueprints/BP_FirstPersonCharacter.BP_FirstPersonCharacter_C|GetAC_Currency _asbp_first_person_character) (+ (Variables|/Game/Blueprints/AC_Currency.AC_Currency_C|GetcurrencyMultiplier (Variables|/Game/FirstPerson/Blueprints/BP_FirstPersonCharacter.BP_FirstPersonCharacter_C|GetAC_Currency _asbp_first_person_character)) 1))
  (Default|RemoveCurrency (Variables|/Game/FirstPerson/Blueprints/BP_FirstPersonCharacter.BP_FirstPersonCharacter_C|GetAC_Currency _asbp_first_person_character) (Variables|Default|GetatomValueCost))
  (Variables|Default|SetatomValueUpgrades (+ (Variables|Default|GetatomValueUpgrades) 1))
  (Variables|Default|SetatomValueCost (* (Variables|Default|GetatomValueCost) 3.0)))

(fn PlayerHasEnough
  (params (upgradeCost :type Float%20%28double-precision%29))
  (bind _asbp_first_person_character (Utilities|Casting|CastToBP_FirstPersonCharacter (Game|GetPlayerCharacter 0)))
  (if (>= (Variables|/Game/Blueprints/AC_Currency.AC_Currency_C|Getcurrency (Variables|/Game/FirstPerson/Blueprints/BP_FirstPersonCharacter.BP_FirstPersonCharacter_C|GetAC_Currency _asbp_first_person_character)) upgradeCost)
    (return true)
    (else
      (return false))))